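; BP_Berry is a collectible berry that the player picks up by touching it.
; When BP_Player overlaps its collision sphere, it increments the player's BerriesCollected count, plays a pickup sound and destroys itself.
; Once that count reaches at least three, it changes the CurrentGameState on BP_GameMode and plays the Gameover sound.
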(event OnComponentBeginOverlap(Sphere_Collision)
  (params (OverlappedComponent :type Primitive%20Component%20Object%20Reference) (OtherActor :type Actor%20Object%20Reference) (OtherComp :type Primitive%20Component%20Object%20Reference) (OtherBodyIndex :type Integer) (bFromSweep :type Boolean) (SweepResult :type Hit%20Result%20Structure%20%28by%20ref%29))
  (bind _asbp_player (Utilities|Casting|CastToBP_Player OtherActor))
  (bind _result (Math|Integer|IncrementInt (Variables|/Game/Fab/Duck_-_NPR/Blueprints/BP_Player.BP_Player_C|GetberriesCollected _asbp_player))
    (:%20%20
      (bind _output_get (Variables|/Game/Fab/Duck_-_NPR/Blueprints/BP_Player.BP_Player_C|SetberriesCollected _asbp_player _result))
      (Audio|PlaySound2D "/Game/myFolder/Level_Assets/Sounds/berryPickedUpSFX.berryPickedUpSFX" 1.0 1.0 0.0 0 0)
      (Actor|DestroyActor)
      (if (>= _output_get 3)
        (bind _asbp_game_mode (Utilities|Casting|CastToBP_GameMode (Game|GetGameMode)))
        (Variables|/Game/myFolder/Level_Assets/Blueprints/BP_GameMode.BP_GameMode_C|SetcurrentGameState _asbp_game_mode "NewEnumerator3")
        (Audio|PlaySound2D "/Game/myFolder/Level_Assets/Sounds/gameover.gameover" 1.0 1.0 0.0 0 0)))))

(event EventBeginPlay)

(event Collision|EventActorBeginOverlap
  (params (OtherActor :type Actor%20Object%20Reference)))

(event EventTick
  (params (DeltaSeconds :type Float%20%28single-precision%29)))

(fn ConstructionScript)